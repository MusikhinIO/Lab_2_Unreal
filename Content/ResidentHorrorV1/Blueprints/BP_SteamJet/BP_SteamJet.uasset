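; BP_SteamJet is a one-shot steam jet that goes off when the player character enters its trigger sphere.
; The sphere overlap checks for the player and a Used flag, then calls the SteamJet event.
; That event activates the Niagara effect, disables the sphere's collision, plays the steam sound cue and prints a debug "Hello".
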(event OnComponentBeginOverlap(Sphere)
  (params (OverlappedComponent :type Primitive%20Component%20Object%20Reference) (OtherActor :type Actor%20Object%20Reference) (OtherComp :type Primitive%20Component%20Object%20Reference) (OtherBodyIndex :type Integer) (bFromSweep :type Boolean) (SweepResult :type Hit%20Result%20Structure%20%28by%20ref%29))
  (if (and (== OtherActor (CallFunction|MyCharacterResidentHorror)) (not (Variables|Default|GetbUsed?)))
    (Variables|Default|SetbUsed? true)
    (CallFunction|SteamJet)))

(event Custom|SteamJet
  (Components|Activation|Activate (Variables|Default|GetNiagara) true)
  (Collision|SetCollisionEnabled (Variables|Default|GetSphere) "NoCollision")
  (Audio|Components|Audio|Play (Variables|Default|GetCUE_SteamJet) 0.0)
  (Development|PrintString "Hello"))

(fn ConstructionScript)