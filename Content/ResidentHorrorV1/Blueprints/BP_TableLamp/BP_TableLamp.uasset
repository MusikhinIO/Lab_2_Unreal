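; BP_TableLamp is an interactive table lamp that toggles on and off through its InteractItem event.
; The construction script caches dynamic material instances for two slots of the static mesh, then applies the current state, which InteractItem later flips.
; UpdateVisualEffects sets both point lights' visibility and the materials' emissive-style Intensity parameters together.
; The LightsOff flag reads inverted: true means the lamp is lit.
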(event Custom|UpdateVisualEffects
  (Rendering|SetVisibility (Variables|Default|GetPointLight) (Variables|Default|GetLightsOff) false)
  (if (Variables|Default|GetLightsOff)
    (Rendering|Material|SetScalarParameterValue (Variables|Default|GetLamp) "Intensity" 1.0 :!class /Script/Engine.MaterialInstanceDynamic)
    (Rendering|Material|SetScalarParameterValue (Variables|Default|GetLampLight) "Intensity" 4.0 :!class /Script/Engine.MaterialInstanceDynamic)
    (else
      (Rendering|Material|SetScalarParameterValue (Variables|Default|GetLamp) "Intensity" 0.0 :!class /Script/Engine.MaterialInstanceDynamic))))

(event EventInteractItem
  (params (ACTO :type Actor%20Object%20Reference) (Player :type BP%20Resident%20Horror%20V1%20Object%20Reference))
  (if (Variables|Default|GetLightsOff)
    (Variables|Default|SetLightsOff false)
    (else
      (Variables|Default|SetLightsOff true)))
  (CallFunction|UpdateVisualEffects))

(fn ConstructionScript
  (|CallParentFunction)
  (CallFunction|CacheMaterialInst)
  (CallFunction|UpdateVisualEffects))

(fn CacheMaterialInst
  (bind _returnvalue (Rendering|Material|CreateDynamicMaterialInstance (Variables|Default|GetStaticMesh) 1 "/Game/ResidentHorrorV1/Demo/Materials/M_TableLamp_Base.M_TableLamp_Base" "None" :!class /Script/Engine.PrimitiveComponent))
  (Variables|Default|SetLamp _returnvalue)
  (bind _returnvalue_2 (Rendering|Material|CreateDynamicMaterialInstance (Variables|Default|GetStaticMesh) 0 "/Game/ResidentHorrorV1/Demo/Materials/M_TableLamp_Lamp.M_TableLamp_Lamp" "None" :!class /Script/Engine.PrimitiveComponent))
  (Variables|Default|SetLampLight _returnvalue_2))